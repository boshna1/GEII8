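; BP_RoadGenerator places pooled traffic cars near the player, with no road-building logic in this file.
; On BeginPlay it caches the level's BP_CarPool and BP_Player.
; GenerateNewCar, not called here, takes a SlowCar or FuelCar from the pool, teleports it to a random offset from the player and calls its OnSpawnMessage.
; The random pick uses a max of 1, so it always yields SlowCar.
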(event EventBeginPlay
  (bind _returnvalue (Actor|GetActorOfClass "/Game/Blueprints/BP_CarPool.BP_CarPool_C"))
  (Variables|Default|SetCarPool _returnvalue)
  (bind _returnvalue_2 (Actor|GetActorOfClass "/Game/Blueprints/Player/BP_Player.BP_Player_C"))
  (Variables|Default|SetPlayerRef _returnvalue_2))

(event Collision|EventActorBeginOverlap
  (params (OtherActor :type Actor%20Object%20Reference)))

(event EventTick
  (params (DeltaSeconds :type Float%20%28single-precision%29)))

(fn ConstructionScript)

(fn GenerateNewCar
  (bind _returnvalue (Math|Random|RandomFloatinRange 0.0 5e+02))
  (bind _returnvalue_2 (Math|Random|RandomFloatinRange 0.0 5e+01))
  (bind _carpool (Variables|Default|GetCarPool))
  (bind _playerref (Variables|Default|GetPlayerRef))
  (bind _returnvalue_3 (Math|Vector|MakeVector _returnvalue _returnvalue_2 5e+01))
  (bind _returnvalue_4 (Transformation|GetActorLocation _playerref))
  (bind _returnvalue_5 (+ _returnvalue_4 _returnvalue_3))
  (if (== (Math|Random|RandomInteger 1) 0)
    (bind _car (Default|GetAvailable _carpool "SlowCar"))
    (Transformation|SetActorLocation _car _returnvalue_5 false true)
    (Class|BPIPool|OnSpawn(Message) _car)
    (else
      (bind _car_2 (Default|GetAvailable _carpool "FuelCar"))
      (Transformation|SetActorLocation _car_2 _returnvalue_5 false true)
      (Class|BPIPool|OnSpawn(Message) _car_2))))