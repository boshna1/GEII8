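; BP_Player is the player-driven character in a driving game with fuel, score and a finish line.
; Enhanced Input moves it and adds score while held, as Tick drains fuel during driving and updates the UI widget.
; A state function sets walk speed for normal, slowed or out-of-fuel.
; Cube overlaps use actor tags to refuel or briefly slow the player, despawn those cars, and print at the finish.
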(event OnComponentBeginOverlap(Cube)
  (params (OverlappedComponent :type Primitive%20Component%20Object%20Reference) (OtherActor :type Actor%20Object%20Reference) (OtherComp :type Primitive%20Component%20Object%20Reference) (OtherBodyIndex :type Integer) (bFromSweep :type Boolean) (SweepResult :type Hit%20Result%20Structure%20%28by%20ref%29))
  (Utilities|FlowControl|Sequence
    (:then_0
      (if (Actor|ActorHasTag OtherActor "FuelCar")
        (CallFunction|FuelUp)
        (bind _asbp_fuel_car (Utilities|Casting|CastToBP_FuelCar OtherActor))
        (Default|OnDespawn _asbp_fuel_car)))
    (:then_1
      (if (Actor|ActorHasTag OtherActor "SlowCar")
        (CallFunction|SlowDown)
        (bind _asbp_slow_car (Utilities|Casting|CastToBP_SlowCar OtherActor))
        (Default|OnDespawn _asbp_slow_car)))
    (:then_2
      (if (Actor|ActorHasTag OtherActor "FinishLine")
        (Development|PrintString "Finish!")))))

(event Custom|ResetState
  (CallFunction|SetState "NewEnumerator0"))

(event Input|EnhancedActionEvents|EnhancedInputActionIA_Move
  (params (ActionValue :type Vector%202D%20Structure) (ElapsedSeconds :type Float%20%28double-precision%29) (TriggeredSeconds :type Float%20%28double-precision%29) (InputAction :type Input%20Action%20Object%20Reference :default "/Game/Blueprints/Player/IA_Move.IA_Move"))
  (bind (_x _y) (Math|Vector2D|BreakVector2D ActionValue))
  (:Triggered
    (Pawn|Input|AddMovementInput (Math|Vector|GetRightVector (Variables|Collision|GetCapsuleComponent)) _x false)
    (Pawn|Input|AddMovementInput (Math|Vector|GetForwardVector (Variables|Collision|GetCapsuleComponent)) _y false)
    (bind _output_get (Variables|Default|SetPoints (+ (Variables|Default|GetPoints) 1.0)))
    (Variables|/Script/UMG.TextBlock|SetText (Variables|/Game/Blueprints/Player/BPW_UI.BPW_UI_C|GetScore (Variables|Default|GetUIRef)) (Utilities|Text|ToText(Float) _output_get "HalfToEven")))
  (:Started
    (Variables|Default|SetDriving true))
  (:Completed
    (Variables|Default|SetDriving false)))

(event EventBeginPlay
  (bind _asplayer_controller (Utilities|Casting|CastToPlayerController (Game|GetPlayerController 0)))
  (Utilities|IsValid (PlayerController|LocalPlayerSubsystems|GetEnhancedInputLocalPlayerSubsystem _asplayer_controller)
    (:Is%20Valid
      (Input|AddMappingContext (PlayerController|LocalPlayerSubsystems|GetEnhancedInputLocalPlayerSubsystem _asplayer_controller) "/Game/Blueprints/Player/IMC_Player.IMC_Player" 0 "(bIgnoreAllPressedKeysUntilRelease=True,bForceImmediately=False,bNotifyUserSettings=False)")
      (Variables|/Script/Engine.CharacterMovementComponent|SetMaxWalkSpeed (Variables|Character|GetCharacterMovement) (Variables|Default|GetSpeed))
      (bind _returnvalue (UserInterface|CreateWidget "/Game/Blueprints/Player/BPW_UI.BPW_UI_C" (Game|GetPlayerController 0)))
      (Variables|Default|SetUIRef _returnvalue))))

(event Collision|EventActorBeginOverlap
  (params (OtherActor :type Actor%20Object%20Reference)))

(event EventTick
  (params (DeltaSeconds :type Float%20%28single-precision%29))
  (Utilities|FlowControl|Sequence
    (:then_0
      (bind _output_get (Variables|/Script/Engine.CharacterMovementComponent|SetMaxWalkSpeed (Variables|Character|GetCharacterMovement) (Variables|Default|GetSpeed)))
      (Variables|/Script/UMG.TextBlock|SetText (Variables|/Game/Blueprints/Player/BPW_UI.BPW_UI_C|GetSpeed (Variables|Default|GetUIRef)) (Utilities|Text|ToText(Float) _output_get "HalfToEven")))
    (:then_1
      (if (<= (Variables|Default|GetFuel) 0.0)
        (CallFunction|SetState "NewEnumerator2")))
    (:then_2
      (if (Variables|Default|GetDriving)
        (if (not (<= (Variables|Default|GetFuel) 0.0))
          (bind _output_get_2 (Variables|Default|SetFuel (- (Variables|Default|GetFuel) 1e+01)))
          (Variables|/Script/UMG.TextBlock|SetText (Variables|/Game/Blueprints/Player/BPW_UI.BPW_UI_C|GetFuel (Variables|Default|GetUIRef)) (Utilities|Text|ToText(Float) _output_get_2 "HalfToEven")))))))

(event EventFuelUp
  (Variables|Default|SetFuel (+ (Variables|Default|GetFuel) 5e+02)))

(event EventSlowDown
  (CallFunction|SetState "NewEnumerator1")
  (Utilities|Time|SetTimerbyEvent (delegate Custom|ResetState) 1.5))

(fn ConstructionScript)

(fn SetState
  (params (State :type ESpeedState%20Enum :default "NewEnumerator0"))
  (bind _output_get (Variables|Default|SetCurrentState State))
  (switch Utilities|FlowControl|Switch|SwitchonESpeedState _output_get
    (:NewEnumerator0
      (Variables|Default|SetSpeed 1e+03))
    (:NewEnumerator1
      (Variables|Default|SetSpeed 4e+02))
    (:NewEnumerator2
      (Variables|Default|SetSpeed 0.0))))